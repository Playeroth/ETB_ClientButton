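; Actor component that makes its owner interactable by using a spawned BP_Latch as a proxy input.
; On BeginPlay the server spawns the latch with replicated primitives, optionally hidden, and attaches it at a relative transform.
; While enabled, Tick detects reversals in the latch's X1 value, flips IsToggled and fires OnInteracted according to UseType.
; StartType sets the initial state, and disabling interaction scales the latch to zero.
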(event EventBeginPlay
  (Variables|Default|SetActorOwner (Components|GetOwner))
  (if (Networking|IsServer)
    (bind _returnvalue (Game|SpawnActorfromClass "/Game/Interactables/BP_Latch.BP_Latch_C" (Transformation|GetActorTransform (Variables|Default|GetActorOwner)) "AlwaysSpawn" 0 0))
    (Class|ActorComponent|SetIsReplicated (Actor|GetComponentsByClass _returnvalue "/Script/Engine.PrimitiveComponent") true)
    (Collision|SetCollisionResponsetoChannel (Actor|GetComponentsByClass _returnvalue "/Script/Engine.PrimitiveComponent") "ECC_Destructible" "ECR_Ignore")
    (bind _output_get (Variables|Default|SetLatch_CheckInteractable _returnvalue))
    (Rendering|SetVisibility (Variables|/Script/Engine.Actor|GetRootComponent _output_get) (not (Variables|Default|GetisCompHidden)) true)
    (CallFunction|CheckStartInteract)
    (CallFunction|BeginValidActorOwner)))

(event EventTick
  (params (DeltaSeconds :type Float%20%28single-precision%29))
  (if (Variables|Default|GetisCompInteractEnabled)
    (Utilities|CheckonInteracted
      (:Interacted
        (Variables|Default|SetwasUsed true)
        (CallFunction|CheckonUse)))))

(event EventEndPlay
  (params (EndPlayReason :type EEndPlayReason%20Enum :default "Destroyed"))
  (Actor|SetLifeSpan (Variables|Default|GetLatch_CheckInteractable) 0.01)
  (Default|CallOnEndPlay self (Variables|Default|GetActorOwner)))

(fn BeginViewStaticMesh
  (if (Variables|Default|GetDebug_isInteractVisible)
    (for _array_element (Actor|GetComponentsByClass (Variables|Default|GetActorOwner) "/Script/Engine.PrimitiveComponent")
      (Rendering|Material|SetMaterial _array_element 0 "/Engine/EngineDebugMaterials/WireframeMaterial.WireframeMaterial"))
    (for _array_element_2 (Actor|GetComponentsByClass (Variables|Default|GetLatch_CheckInteractable) "/Script/Engine.PrimitiveComponent")
      (Rendering|Material|SetMaterial _array_element_2 0 "/Engine/EngineDebugMaterials/WireframeMaterial.WireframeMaterial"))))

(fn BeginValidActorOwner
  (bind _transfromrelativetoowner (Variables|Default|GetTransfromRelativeToOwner))
  (bind _latch_checkinteractable (Variables|Default|GetLatch_CheckInteractable))
  (bind (_x _y _z) (Math|Vector|BreakVector (.location _transfromrelativetoowner)))
  (Utilities|IsValid (Variables|Default|GetActorOwner)
    (:Is%20Valid
      (Transformation|AttachActorToActor _latch_checkinteractable (Variables|Default|GetActorOwner) "None" "SnapToTarget" "SnapToTarget" "SnapToTarget" true)
      (Transformation|SetRelativeTransform (Variables|/Script/Engine.Actor|GetRootComponent _latch_checkinteractable) (Math|Transform|MakeTransform (Math|Vector|MakeVector (+ _x -5.0) _y _z) (.rotation _transfromrelativetoowner) (.scale _transfromrelativetoowner)) false false))))

(fn ToggleCanInteract
  (params (isEnabled :type Boolean))
  (bind _latch_checkinteractable (Variables|Default|GetLatch_CheckInteractable))
  (bind _returnvalue (Transformation|GetActorScale3D _latch_checkinteractable))
  (if (Math|Vector|VectorIsZero _returnvalue)
    _
    (else
      (Variables|Default|SetDefaultScale _returnvalue)))
  (if isEnabled
    (Transformation|SetActorScale3D _latch_checkinteractable (Variables|Default|GetDefaultScale))
    (Variables|Default|SetisCompInteractEnabled true)
    (else
      (Transformation|SetActorScale3D _latch_checkinteractable "0, 0, 0")
      (Variables|Default|SetisCompInteractEnabled false))))

(fn CallonInteract
  (Default|CallOnInteracted (Variables|Default|GetisToggled) (Variables|Default|GetActorOwner) (Variables|Default|GetID) self))

(fn CheckStartInteract
  (switch Utilities|FlowControl|Switch|SwitchonInteractType (Variables|Default|GetStartType)
    (:NewEnumerator2
      (LocalVariables|SetStartInteract true)
      (CallFunction|ToggleCanInteract (LocalVariables|GetStartInteract) :!label _label))
    (:NewEnumerator0
      (LocalVariables|SetStartInteract false)
      (goto _label))
    (:NewEnumerator1
      (Variables|Default|SetisCompInteractEnabled false))))

(fn CheckonUse
  (switch Utilities|FlowControl|Switch|SwitchonUseType (Variables|Default|GetUseType)
    (:NewEnumerator2
      (CallFunction|CallonInteract))
    (:NewEnumerator0
      (CallFunction|ToggleCanInteract false)
      (CallFunction|CallonInteract))
    (:NewEnumerator1
      (Variables|Default|SetisCompInteractEnabled false)
      (CallFunction|CallonInteract))))