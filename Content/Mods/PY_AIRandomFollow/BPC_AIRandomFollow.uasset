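; Mod component that drives an AI pawn to wander to random reachable points or seek the nearest player character.
; Tick checks the current path, using a randomized delay, weighted chance or always-chase flag to issue AIMoveTo.
; Starting a chase swaps the attached actor for a chase object, and wandering restores it.
; An optional walk-speed change is reapplied every tick, and an optional retriggerable timer removes the component.
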(event Custom|GoToActor
  (params (ActorToSeek :type Actor%20Object%20Reference))
  (bind _onchaseplayerobject (Variables|Default|GetOnChasePlayerObject))
  (AI|AIMoveTo (AI|GetAIController (Variables|Default|GetEntityPawn)) "0, 0, 0" ActorToSeek (Variables|Default|GetAcceptanceRadius) "Default" "Default" true (Variables|Default|GetForceAILock)
    (:then
      (if (Utilities|IsValidClass _onchaseplayerobject)
        (bind _returnvalue (Game|SpawnActorfromClass _onchaseplayerobject (Math|Transform|MakeTransform "0, 0, 0" "0, 0, 0" "1,1,1") "AlwaysSpawn" 0 0))
        (bind _output_get (Variables|Default|SetChasePlayerRef _returnvalue))
        (Transformation|AttachActorToActor _output_get (Variables|Default|GetEntityPawn) "None" "SnapToTarget" "SnapToTarget" "SnapToTarget" true)
        (Variables|Default|SetObjectToAttachClass (Utilities|GetClass (Variables|Default|GetObject%20To%20Attach)))
        (Actor|SetLifeSpan (Variables|Default|GetObject%20To%20Attach) 0.01)))))

(event Custom|GoToRandom
  (params (LocationToGo :type Vector))
  (AI|AIMoveTo (AI|GetAIController (Variables|Default|GetEntityPawn)) LocationToGo 0 (Variables|Default|GetAcceptanceRadius) "Default" "Default" true (Variables|Default|GetForceAILock)
    (:then
      (Utilities|IsValid (Variables|Default|GetChasePlayerRef)
        (:Is%20Valid
          (Actor|SetLifeSpan (Variables|Default|GetChasePlayerRef) 0.01)
          (bind _returnvalue (Game|SpawnActorfromClass (Variables|Default|GetObjectToAttachClass) (Math|Transform|MakeTransform "0, 0, 0" "0, 0, 0" "1,1,1") "AlwaysSpawn" 0 0))
          (bind _output_get (Variables|Default|SetObject%20To%20Attach _returnvalue))
          (Transformation|AttachActorToActor _output_get (Variables|Default|GetEntityPawn) "None" "SnapToTarget" "SnapToTarget" "SnapToTarget" true))))))

(event Custom|RetriggerDelayToDeletion
  (if (not (== (Variables|Default|GetDelayToDeleteComp) -1.0))
    (Utilities|FlowControl|RetriggerableDelay (Variables|Default|GetDelayToDeleteComp))
    (Components|DestroyComponent)))

(event EventBeginPlay
  (bind _aspawn (Utilities|Casting|CastToPawn (Components|GetOwner)))
  (Variables|Default|SetEntityPawn _aspawn)
  (Utilities|FlowControl|Sequence
    (:then_0
      (CallFunction|BeginConfigSpeed)
      (bind _object_to_attach (Variables|Default|GetObject%20To%20Attach)
        (:then
          (Transformation|AttachActorToActor _object_to_attach (Variables|Default|GetEntityPawn) "None" "SnapToTarget" "SnapToTarget" "SnapToTarget" true))
        (:else)))
    (:then_1
      (if (not (== (Variables|Default|GetDelayToDeleteComp) -1.0))
        (CallFunction|RetriggerDelaytoDeletion)))))

(event EventTick
  (params (DeltaSeconds :type Float%20%28single-precision%29))
  (bind _chancetogonearplayer (Variables|Default|GetChanceToGoNearPlayer))
  (Utilities|FlowControl|Sequence
    (:then_0
      (if (Utilities|IsValid (Class|AIBlueprintHelperLibrary|GetCurrentPath (AI|GetAIController (Variables|Default|GetEntityPawn))))
        (Utilities|FlowControl|Delay (+ (Variables|Default|GetTimeToResetAI) (Math|Random|RandomFloatinRange 0.0 2.5)))
        (if (!= _chancetogonearplayer -1.0) :!label _label
          (if (Math|Random|RandomBoolwithWeight _chancetogonearplayer)
            (CallFunction|GetNearestPlayer)
            (else
              (CallFunction|GotoRandom (CallFunction|GetRandomLocation) :!label _label_2)))
          (else
            (goto _label_2)))
        (elif (Variables|Default|GetisAlwaysGoNearPlayer)
          (CallFunction|GetNearestPlayer)
          (else
            (goto _label)))))
    (:then_1
      (CallFunction|ForceSpeed))))

(event EventEndPlay
  (params (EndPlayReason :type EEndPlayReason%20Enum :default "Destroyed"))
  (Actor|DestroyActor (Variables|Default|GetObject%20To%20Attach))
  (Actor|DestroyActor (Variables|Default|GetChasePlayerRef)))

(fn GetNearestPlayer
  (bind _outactors (Actor|GetAllActorsOfClass "/Game/Game/BPCharacter_Demo.BPCharacter_Demo_C"))
  (CallFunction|GotoActor (.ReturnValue (Actor|FindNearestActor (Transformation|GetActorLocation (Variables|Default|GetEntityPawn)) _outactors))))

(fn GetRandomLocation
  (bind _locationsearchforrandomdistance (Variables|Default|GetLocationSearchForRandomDistance))
  (return (.RandomLocation (AI|Navigation|GetRandomReachablePointinRadius (select (Math|Vector|Equal(Vector) _locationsearchforrandomdistance "-1.000000,-1.000000,-1.000000" 0.0001) (Transformation|GetActorLocation (Variables|Default|GetEntityPawn)) _locationsearchforrandomdistance) (Variables|Default|GetRandomRadiusReachable) 0 0))))

(fn BeginConfigSpeed
  (if (!= (Variables|Default|GetCustomSpeed) -1.0)
    (bind _ascharacter (Utilities|Casting|CastToCharacter (Variables|Default|GetEntityPawn)))
    (bind _output_get (Variables|Default|SetAsCharacter _ascharacter))
    (switch Utilities|FlowControl|Switch|SwitchonAISpeedType (Variables|Default|GetSpeedType)
      (:NewEnumerator2
        (bind _output_get_2 (Variables|/Script/Engine.CharacterMovementComponent|SetMaxWalkSpeed (Variables|/Script/Engine.Character|GetCharacterMovement _output_get) (Variables|Default|GetCustomSpeed)))
        (Variables|Default|SetCurrentSpeed _output_get_2))
      (:NewEnumerator0
        (bind _output_get_3 (Variables|/Script/Engine.CharacterMovementComponent|SetMaxWalkSpeed (Variables|/Script/Engine.Character|GetCharacterMovement _output_get) (+ (Variables|/Script/Engine.CharacterMovementComponent|GetMaxWalkSpeed (Variables|/Script/Engine.Character|GetCharacterMovement _output_get)) (Variables|Default|GetCustomSpeed))))
        (Variables|Default|SetCurrentSpeed _output_get_3))
      (:NewEnumerator1
        (bind _output_get_4 (Variables|/Script/Engine.CharacterMovementComponent|SetMaxWalkSpeed (Variables|/Script/Engine.Character|GetCharacterMovement _output_get) (* (Variables|/Script/Engine.CharacterMovementComponent|GetMaxWalkSpeed (Variables|/Script/Engine.Character|GetCharacterMovement _output_get)) (Variables|Default|GetCustomSpeed))))
        (Variables|Default|SetCurrentSpeed _output_get_4)))))

(fn ForceSpeed
  (if (!= (Variables|Default|GetCustomSpeed) -1.0)
    (Variables|/Script/Engine.CharacterMovementComponent|SetMaxWalkSpeed (Variables|/Script/Engine.Character|GetCharacterMovement (Variables|Default|GetAsCharacter)) (Variables|Default|GetCurrentSpeed))))